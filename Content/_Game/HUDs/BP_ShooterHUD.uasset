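; Shooter HUD that draws a dynamic crosshair at screen center, made of a center dot and four separate textured pieces.
; BeginPlay caches the player pawn as BP_ShooterCharacter, and DrawHUD re-casts it whenever that reference is invalid.
; Each frame DrawHUD reads the character's crosshair spread and scales it by a max spread to push the top, bottom, left and right pieces outward.
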(event EventBeginPlay
  ;[1 1 1] Setting Shooter Character refrence
  (Utilities|IsValid (Variables|Default|GetShooterCharacter)
    (:Is%20Valid
      _)
    (:Is%20Not%20Valid
      _))
  (bind _asbp_shooter_character (Utilities|Casting|CastToBP_ShooterCharacter (Game|Player|GetPlayerPawn 0)))
  (Variables|Default|SetShooterCharacter _asbp_shooter_character))

(event Collision|EventActorBeginOverlap
  (params (OtherActor :type Actor%20Object%20Reference)))

(event EventTick
  (params (DeltaSeconds :type Float%20%28single-precision%29)))

(event EventDrawHUD
  (params (SizeX :type Integer) (SizeY :type Integer))
  (bind _crosshairsize (Variables|Default|GetCrosshairSize))
  (bind _crosshairsize_2 (Variables|Default|GetCrosshairSize))
  (bind _crosshairsize_3 (Variables|Default|GetCrosshairSize))
  (bind _crosshairsize_4 (Variables|Default|GetCrosshairSize))
  ;[1 1 1] Set Screen Center
  (Variables|Default|SetScreeCenter (Math|Vector2D|MakeVector2D (Math|Conversions|ToFloat(Integer) (/ SizeX 2)) (Math|Conversions|ToFloat(Integer) (/ SizeY 2))))
  ;[1 1 1] Setting CrosshairSpreadMultiplier
  (Utilities|IsValid (Variables|Default|GetShooterCharacter)
    (:Is%20Valid
      _)
    (:Is%20Not%20Valid
      (bind _asbp_shooter_character (Utilities|Casting|CastToBP_ShooterCharacter (Game|Player|GetPlayerPawn 0)))
      (Variables|Default|SetShooterCharacter _asbp_shooter_character)))
  (Variables|Default|SetcrosshairSpreadMultiplier (Class|ShooterCharacter|GetCrosshairSpread (Variables|Default|GetShooterCharacter)))
  ;[1 1 1] Move X and Y by half crosshair size AND setting crosshairBase
  (Variables|Default|SetcrosshairBase (Math|Vector2D|MakeVector2D (- (.x (Variables|Default|GetScreeCenter)) (Math|Conversions|ToFloat(Integer) (/ (Variables|Default|GetCrosshairSize) 2))) (- (.y (Variables|Default|GetScreeCenter)) (Math|Conversions|ToFloat(Integer) (/ (Variables|Default|GetCrosshairSize) 2)))))
  ;[1 1 1] Drawing Center Dot
  (Canvas|DrawTexture "/Game/_Game/_Assets/Textures/Crosshairs/Crosshair_Dot.Crosshair_Dot" (- (.x (Variables|Default|GetcrosshairBase)) 16.0) (- (.y (Variables|Default|GetcrosshairBase)) 16.0) 64.0 64.0 0.0 0.0 1.0 1.0 "(R=1.000000,G=1.000000,B=1.000000,A=1.000000)")
  ;[1 1 1] Drawing bottom piece of the crosshair
  (Canvas|DrawTexture "/Game/_Game/_Assets/Textures/Crosshairs/Crosshair_Quad_9_Bottom.Crosshair_Quad_9_Bottom" (.x (Variables|Default|GetcrosshairBase)) (+ (.y (Variables|Default|GetcrosshairBase)) (* (Variables|Default|GetcrosshairSpreadMultiplier) (Variables|Default|GetcrossSpreadMax))) (Math|Conversions|ToFloat(Integer) _crosshairsize_3) (Math|Conversions|ToFloat(Integer) _crosshairsize_3) 0.0 0.0 1.0 1.0 "(R=1.000000,G=1.000000,B=1.000000,A=1.000000)")
  ;[1 1 1] Drawing Top piece of the crosshair
  (Canvas|DrawTexture "/Game/_Game/_Assets/Textures/Crosshairs/Crosshair_Quad_9_Top.Crosshair_Quad_9_Top" (.x (Variables|Default|GetcrosshairBase)) (- (.y (Variables|Default|GetcrosshairBase)) (* (Variables|Default|GetcrosshairSpreadMultiplier) (Variables|Default|GetcrossSpreadMax))) (Math|Conversions|ToFloat(Integer) _crosshairsize) (Math|Conversions|ToFloat(Integer) _crosshairsize) 0.0 0.0 1.0 1.0 "(R=1.000000,G=1.000000,B=1.000000,A=1.000000)")
  ;[1 1 1] Drawing Right piece of the crosshair
  (Canvas|DrawTexture "/Game/_Game/_Assets/Textures/Crosshairs/Crosshair_Quad_9_Right.Crosshair_Quad_9_Right" (+ (* (Variables|Default|GetcrosshairSpreadMultiplier) (Variables|Default|GetcrossSpreadMax)) (.x (Variables|Default|GetcrosshairBase))) (.y (Variables|Default|GetcrosshairBase)) (Math|Conversions|ToFloat(Integer) _crosshairsize_2) (Math|Conversions|ToFloat(Integer) _crosshairsize_2) 0.0 0.0 1.0 1.0 "(R=1.000000,G=1.000000,B=1.000000,A=1.000000)")
  ;[1 1 1] Drawing Left piece of the crosshair
  (Canvas|DrawTexture "/Game/_Game/_Assets/Textures/Crosshairs/Crosshair_Quad_9_Left.Crosshair_Quad_9_Left" (- (.x (Variables|Default|GetcrosshairBase)) (* (Variables|Default|GetcrosshairSpreadMultiplier) (Variables|Default|GetcrossSpreadMax))) (.y (Variables|Default|GetcrosshairBase)) (Math|Conversions|ToFloat(Integer) _crosshairsize_4) (Math|Conversions|ToFloat(Integer) _crosshairsize_4) 0.0 0.0 1.0 1.0 "(R=1.000000,G=1.000000,B=1.000000,A=1.000000)"))

(fn ConstructionScript)